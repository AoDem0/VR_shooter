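; BP_Basic is a basic health Blueprint that tracks HP and handles enemy death.
; HP starts at MaxHP on BeginPlay, and TakeDamage subtracts damage, but its zero-HP check leads to no action.
; Die, not called within this graph, asks BP_EnemySpawner to try spawning an enemy, then destroys its owner if that is a BP_Enemie.
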(event `self.ReceiveBeginPlay`
  (set `self.HP` (`self.MaxHP`)))

(fn `Die`
  (bind _returnvalue (`GameplayStatics.GetActorOfClass` "/Game/BP_EnemySpawner.BP_EnemySpawner_C"))
  (`/Game/BP_EnemySpawner.TrySpawnEnemy` _returnvalue)
  (bind _asbp_enemie (cast `/Game/Characters/BP_Enemie` (`self.GetOwner` self)))
  (`Actor.K2_DestroyActor` _asbp_enemie))

(fn `TakeDamage`
  (params (DamageDealt :type "Float (double-precision)"))
  (bind _output_get (set `self.HP` (- (`self.HP`) DamageDealt)))
  (if (<= _output_get 0.0)
    _))